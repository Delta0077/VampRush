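; Endless-runner ground tile that populates three lanes with obstacles or coins on BeginPlay.
; Each lane runs cascading chance checks with a fresh random roll each time; side lanes can get broken barriers, the middle cannot.
; When the player character overlaps the Box, it has the GameMode spawn ground tiles, adds and prints points, multiplies walk speed within a clamp, then destroys itself after a short delay.
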(event `self.ReceiveBeginPlay`
  (`self.Spawn Obstacles`))

(event `self.Box.OnComponentBeginOverlap`
  (params (OverlappedComponent :type "PrimitiveComponent Object Reference") (OtherActor :type "Actor Object Reference") (OtherComp :type "PrimitiveComponent Object Reference") (OtherBodyIndex :type Integer) (bFromSweep :type Boolean) (SweepResult :type "HitResult Structure (by ref)"))
  (cast `/Game/ThirdPersonBP/Blueprints/ThirdPersonCharacter` OtherActor)
  (bind _asthird_person_game_mode (cast `/Game/ThirdPersonBP/Blueprints/ThirdPersonGameMode` (`GameplayStatics.GetGameMode`)))
  (`/Game/ThirdPersonBP/Blueprints/ThirdPersonGameMode.SpawnGroundTiles` _asthird_person_game_mode)
  (bind _asthird_person_game_mode_2 (cast `/Game/ThirdPersonBP/Blueprints/ThirdPersonGameMode` (`GameplayStatics.GetGameMode`)))
  (bind _output_get (set `/Game/ThirdPersonBP/Blueprints/ThirdPersonGameMode.CurrentPoints` (+ (`/Game/ThirdPersonBP/Blueprints/ThirdPersonGameMode.CurrentPoints` _asthird_person_game_mode_2) 100) _asthird_person_game_mode_2))
  (`KismetSystemLibrary.PrintString` (`KismetStringLibrary.Conv_IntToString` _output_get))
  (bind _asthird_person_character (cast `/Game/ThirdPersonBP/Blueprints/ThirdPersonCharacter` (`GameplayStatics.GetPlayerCharacter` 0)))
  (bind _charactermovement (`Character.CharacterMovement` _asthird_person_character))
  (set `CharacterMovementComponent.MaxWalkSpeed` (`KismetMathLibrary.FClamp` (* (`CharacterMovementComponent.MaxWalkSpeed` _charactermovement) (`self.SpeedMultiPilar`)) 600.0 (`self.MaxSpeed`)) _charactermovement)
  (`KismetSystemLibrary.Delay` 0.2)
  (`self.K2_DestroyActor`))

(fn `Spawn Obstacles`
  (bind _returnvalue (`KismetMathLibrary.RandomFloatInRange` 0.0 1.0))
  (bind _returnvalue_2 (`KismetMathLibrary.RandomFloatInRange` 0.0 1.0))
  (bind _returnvalue_3 (`KismetMathLibrary.RandomFloatInRange` 0.0 1.0))
  (bind _returnvalue_4 (`SceneComponent.K2_GetComponentToWorld` (`self.Lane2`)))
  (bind _returnvalue_5 (`SceneComponent.K2_GetComponentToWorld` (`self.Lane0`)))
  (bind _returnvalue_6 (`SceneComponent.K2_GetComponentToWorld` (`self.Lane1`)))
  ;[0.2336 0.2476 1] Lane0 Spawnning actors
  (if (`KismetMathLibrary.InRange_FloatFloat` _returnvalue_3 0.0 0.05)
    _
    (elif (`KismetMathLibrary.InRange_FloatFloat` _returnvalue_3 0.05 0.35)
      (`|SpawnActorFromClass` "/Game/Blueprints/Obstacles/BP_BrokenConcreateBarrier_Left.BP_BrokenConcreateBarrier_Left_C" _returnvalue_5 "Undefined" "OverrideRootScale" null null)
      (elif (`KismetMathLibrary.InRange_FloatFloat` _returnvalue_3 0.35 0.5)
        (`|SpawnActorFromClass` "/Game/Blueprints/Obstacles/BP_RoadBlockBoard.BP_RoadBlockBoard_C" _returnvalue_5 "Undefined" "OverrideRootScale" null null)
        (elif (`KismetMathLibrary.InRange_FloatFloat` _returnvalue_3 0.5 0.7)
          (`|SpawnActorFromClass` "/Game/Blueprints/Obstacles/BP_StoneWall.BP_StoneWall_C" _returnvalue_5 "Undefined" "OverrideRootScale" null null)
          (elif (`KismetMathLibrary.InRange_FloatFloat` _returnvalue_3 0.7)
            (`|SpawnActorFromClass` "/Game/Blueprints/Coin/BP_Coin.BP_Coin_C" _returnvalue_5 "Undefined" "OverrideRootScale" null null))))))
  ;[0 1 0.5795] Lane1 Spawnning actors
  (if (`KismetMathLibrary.InRange_FloatFloat` _returnvalue 0.0 0.05)
    _
    (elif (`KismetMathLibrary.InRange_FloatFloat` _returnvalue 0.05 0.35)
      _
      (elif (`KismetMathLibrary.InRange_FloatFloat` _returnvalue 0.35 0.5)
        (`|SpawnActorFromClass` "/Game/Blueprints/Obstacles/BP_RoadBlockBoard.BP_RoadBlockBoard_C" _returnvalue_6 "Undefined" "OverrideRootScale" null null)
        (elif (`KismetMathLibrary.InRange_FloatFloat` _returnvalue 0.5 0.7)
          (`|SpawnActorFromClass` "/Game/Blueprints/Obstacles/BP_StoneWall.BP_StoneWall_C" _returnvalue_6 "Undefined" "OverrideRootScale" null null)
          (elif (`KismetMathLibrary.InRange_FloatFloat` _returnvalue 0.7)
            (`|SpawnActorFromClass` "/Game/Blueprints/Coin/BP_Coin.BP_Coin_C" _returnvalue_6 "Undefined" "OverrideRootScale" null null))))))
  ;[1 0.1732 0.1235] Lane2 Spawnning actors
  (if (`KismetMathLibrary.InRange_FloatFloat` _returnvalue_2 0.0 0.05)
    _
    (elif (`KismetMathLibrary.InRange_FloatFloat` _returnvalue_2 0.05 0.35)
      (`|SpawnActorFromClass` "/Game/Blueprints/Obstacles/BP_BrokenConcreateBarrier_Right.BP_BrokenConcreateBarrier_Right_C" _returnvalue_4 "Undefined" "OverrideRootScale" null null)
      (elif (`KismetMathLibrary.InRange_FloatFloat` _returnvalue_2 0.35 0.5)
        (`|SpawnActorFromClass` "/Game/Blueprints/Obstacles/BP_RoadBlockBoard.BP_RoadBlockBoard_C" _returnvalue_4 "Undefined" "OverrideRootScale" null null)
        (elif (`KismetMathLibrary.InRange_FloatFloat` _returnvalue_2 0.5 0.7)
          (`|SpawnActorFromClass` "/Game/Blueprints/Obstacles/BP_StoneWall.BP_StoneWall_C" _returnvalue_4 "Undefined" "OverrideRootScale" null null)
          (elif (`KismetMathLibrary.InRange_FloatFloat` _returnvalue_2 0.7)
            (`|SpawnActorFromClass` "/Game/Blueprints/Coin/BP_Coin.BP_Coin_C" _returnvalue_4 "Undefined" "OverrideRootScale" null null)))))))

(fn `UserConstructionScript`)