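; BP_Rocket is a speed boost power-up triggered when a ThirdPersonCharacter overlaps it.
; On overlap it sets the character's SpeedBoostActive flag, raises MaxWalkSpeed and destroys its SpeedUp component.
; A ten-second Delay then sets a hardcoded normal walk speed and clears the flag, with debug prints at both ends.
; The actor itself is never destroyed here, and the overlap has no guard against retriggering.
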(event `self.ReceiveActorBeginOverlap`
  (params (OtherActor :type "Actor Object Reference"))
  (bind _asthird_person_character (cast `/Game/ThirdPersonBP/Blueprints/ThirdPersonCharacter` OtherActor))
  (set `/Game/ThirdPersonBP/Blueprints/ThirdPersonCharacter.SpeedBoostActive` true _asthird_person_character)
  (`KismetSystemLibrary.PrintString` "Speed Boost Activated")
  (bind _charactermovement (`Character.CharacterMovement` _asthird_person_character))
  (set `CharacterMovementComponent.MaxWalkSpeed` 1800.0 _charactermovement)
  (`ActorComponent.K2_DestroyComponent` (`self.SpeedUp`))
  (`KismetSystemLibrary.Delay` 10.0)
  (`KismetSystemLibrary.PrintString` "Speed Boost Deactivated")
  (set `CharacterMovementComponent.MaxWalkSpeed` 600.0 _charactermovement)
  (set `/Game/ThirdPersonBP/Blueprints/ThirdPersonCharacter.SpeedBoostActive` false _asthird_person_character))

(fn `UserConstructionScript`)